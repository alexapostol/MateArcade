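; BP_HiddenCoinsCircle is an interactable that ties a circle of hidden coins to a UI prompt, apparently a quiz.
; At BeginPlay it caches sixteen preview-mesh locations.
; The first rabbit overlap closes a gate, disables player input and opens W_MainWidget with a self reference and UI-only focus.
; SpawnHiddenCoins, not called within this file, spawns coins just below those locations and calls EndQuizz to re-enable player input.
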(event OnComponentBeginOverlap(Sphere)
  (params (OverlappedComponent :type Primitive%20Component%20Object%20Reference) (OtherActor :type Actor%20Object%20Reference) (OtherComp :type Primitive%20Component%20Object%20Reference) (OtherBodyIndex :type Integer) (bFromSweep :type Boolean) (SweepResult :type Hit%20Result%20Structure%20%28by%20ref%29))
  (bind _returnvalue (Game|GetPlayerController 0))
  (Utilities|FlowControl|Gate false :!label _label
    (:Exit
      (bind _asbp_rabbit (Utilities|Casting|CastToBP_Rabbit OtherActor))
      (bind _output_get (Variables|Default|SetPlayerReference _asbp_rabbit))
      (Variables|/Game/PlatformerDevelopmentKit/Characters/Player/Blueprints/BP_Rabbit.BP_Rabbit_C|SetDisableInput? _output_get true)
      (bind _returnvalue_2 (UserInterface|CreateWidget "/Game/StartQuiz/Widgets/W_MainWidget.W_MainWidget_C" _returnvalue true))
      (Variables|/Game/StartQuiz/Widgets/W_MainWidget.W_MainWidget_C|SetHiddenCoinCircle _returnvalue_2 self)
      (UserInterface|Viewport|AddtoViewport _returnvalue_2 0)
      (Input|SetInputModeUIOnly _returnvalue _returnvalue_2 "DoNotLock")
      (Variables|/Script/Engine.PlayerController|SetbShowMouseCursor _returnvalue true)
      (goto _label Close))))

(event Custom|SpawnHiddenCoins
  (for _array_element (Variables|Default|GetCoinLocations)
    (Game|SpawnActorfromClass "/Game/PlatformerDevelopmentKit/Interactables/Blueprints/BP_Coin.BP_Coin_C" (Math|Transform|MakeTransform (- _array_element "0, 0,50.000000") "0, 0, 0" "1,1,1") "Undefined" 0 0)
    (CallFunction|EndQuizz)))

(event Custom|EndQuizz
  (Variables|/Game/PlatformerDevelopmentKit/Characters/Player/Blueprints/BP_Rabbit.BP_Rabbit_C|SetDisableInput? (stale OnComponentBeginOverlap(Sphere) _output_get) false))

(event EventBeginPlay
  (Variables|Default|SetCoinLocations (Utilities|Array|MakeArray (Transformation|GetWorldLocation (Variables|Default|GetSM_CoinPreview01)) (Transformation|GetWorldLocation (Variables|Default|GetSM_CoinPreview02)) (Transformation|GetWorldLocation (Variables|Default|GetSM_CoinPreview03)) (Transformation|GetWorldLocation (Variables|Default|GetSM_CoinPreview04)) (Transformation|GetWorldLocation (Variables|Default|GetSM_CoinPreview05)) (Transformation|GetWorldLocation (Variables|Default|GetSM_CoinPreview06)) (Transformation|GetWorldLocation (Variables|Default|GetSM_CoinPreview07)) (Transformation|GetWorldLocation (Variables|Default|GetSM_CoinPreview08)) (Transformation|GetWorldLocation (Variables|Default|GetSM_CoinPreview09)) (Transformation|GetWorldLocation (Variables|Default|GetSM_CoinPreview010)) (Transformation|GetWorldLocation (Variables|Default|GetSM_CoinPreview011)) (Transformation|GetWorldLocation (Variables|Default|GetSM_CoinPreview012)) (Transformation|GetWorldLocation (Variables|Default|GetSM_CoinPreview013)) (Transformation|GetWorldLocation (Variables|Default|GetSM_CoinPreview014)) (Transformation|GetWorldLocation (Variables|Default|GetSM_CoinPreview015)) (Transformation|GetWorldLocation (Variables|Default|GetSM_CoinPreview016)))))

(fn ConstructionScript)